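; BP_ExplosiveBarrel is a shootable barrel that explodes and damages nearby objects when its health runs out.
; OnShot passes damage to BarrelHealth, which adds it to health, clamps the result and branches at zero.
; At zero it enables the Sphere's collision, removes the barrel, activates Niagara and destroys the actor after a short delay.
; Sphere overlaps send a fixed negative OnDamaged value to BPI_Damageable actors; debug prints remain.
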(event OnComponentBeginOverlap(Sphere)
  (params (OverlappedComponent :type Primitive%20Component%20Object%20Reference) (OtherActor :type Actor%20Object%20Reference) (OtherComp :type Primitive%20Component%20Object%20Reference) (OtherBodyIndex :type Integer) (bFromSweep :type Boolean) (SweepResult :type Hit%20Result%20Structure%20%28by%20ref%29))
  (if (Utilities|DoesObjectImplementInterface OtherActor "/Game/MyAssets/BPI_Damageable.BPI_Damageable_C")
    (Class|BPIDamageable|OnDamaged(Message) OtherActor -6e+01)
    (Development|PrintString "Hello")))

(event EventBeginPlay
  (|CallParentFunction) ; This node is disabled and will not be called.\nDrag off pins to build functionality.
)

(event Collision|EventActorBeginOverlap
  (params (OtherActor :type Actor%20Object%20Reference))
  (|CallParentFunction OtherActor) ; This node is disabled and will not be called.\nDrag off pins to build functionality.
)

(event EventTick
  (params (DeltaSeconds :type Float%20%28single-precision%29))
  (|CallParentFunction DeltaSeconds) ; This node is disabled and will not be called.\nDrag off pins to build functionality.
)

(event EventOnShot
  (params (DirectionShoot :type Vector :default "0, 0, 0") (Damage :type Float%20%28double-precision%29))
  (Utilities|BarrelHealth Damage
    (:True
      (Development|PrintString "BOMBA")
      (Collision|SetCollisionEnabled (Variables|Default|GetSphere) "QueryAndPhysics")
      (Components|DestroyComponent (Variables|Default|GetBarrel))
      (Components|Activation|Activate (Variables|Default|GetNiagara) false)
      (Utilities|FlowControl|Delay 0.8)
      (Actor|DestroyActor))))

(fn ConstructionScript
  (|CallParentFunction))