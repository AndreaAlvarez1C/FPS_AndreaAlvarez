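; BP_TinCan is a tin can prop that gets knocked around by physics impulses when interacted with or shot.
; Interacting calls the parent handler, then pushes the mesh along the forward vector of Ashe's camera boom with a fixed upward lift.
; A shot pushes it along the shot's horizontal direction with a higher upward kick, ignoring the shot's vertical component.
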(event EventBeginPlay
  (|CallParentFunction) ; This node is disabled and will not be called.\nDrag off pins to build functionality.
)

(event Collision|EventActorBeginOverlap
  (params (OtherActor :type Actor%20Object%20Reference))
  (|CallParentFunction OtherActor) ; This node is disabled and will not be called.\nDrag off pins to build functionality.
)

(event EventTick
  (params (DeltaSeconds :type Float%20%28single-precision%29))
  (|CallParentFunction DeltaSeconds) ; This node is disabled and will not be called.\nDrag off pins to build functionality.
)

(event EventOnInteract
  (bind _ashe (Variables|Default|GetAshe))
  (bind _cameraboom (Variables|/Game/ThirdPerson/Blueprints/BP_ThirdPersonCharacter.BP_ThirdPersonCharacter_C|GetCameraBoom _ashe))
  (bind _returnvalue (Math|Vector|GetForwardVector _cameraboom))
  (bind _returnvalue_2 (* _returnvalue 1e+04))
  (|CallParentFunction)
  (Physics|AddImpulse (Variables|Character|GetMesh) (Math|Vector|MakeVector (.x _returnvalue_2) (.y _returnvalue_2) 2e+03) "None" false))

(event EventOnShot
  (params (DirectionShoot :type Vector :default "0, 0, 0"))
  (Physics|AddImpulse (Variables|Character|GetMesh) (Math|Vector|MakeVector (* (.x DirectionShoot) 3e+03) (* (.y DirectionShoot) 3e+03) 6e+03) "None" false))

(fn ConstructionScript
  (|CallParentFunction))