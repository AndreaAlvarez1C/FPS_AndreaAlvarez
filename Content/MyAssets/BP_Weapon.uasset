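; Player weapon actor that fires BP_Projectile from its Muzzle along the ThirdPersonCharacter's camera direction.
; Shoot routes basic, special and ultimate attacks through DoOnce cooldown gates and CheckAmmo costs.
; Basic counts shots toward a triple burst, resetting after a pause; special fires an angled fan, and ultimate a single projectile.
; Reload, blocked while aiming, refills the magazine from the character's reserve ammo, delaying only full refills.
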(event Custom|ProjectileBasic
  ;[0.3763 0.0185 0.04092 0.5373] Attack Basic
  ;;[0.15 0.15 0.15 0.5] SPAWN DE PROYECTILES ROTACION Y DIRECCION
  (Game|SpawnActorfromClass "/Game/MyAssets/BP_Projectile.BP_Projectile_C" (Math|Transform|MakeTransform (Transformation|GetWorldLocation (Variables|Default|GetMuzzle)) (Math|Conversions|RotationFromXVector (Math|Vector|GetForwardVector (Variables|/Game/ThirdPerson/Blueprints/BP_ThirdPersonCharacter.BP_ThirdPersonCharacter_C|GetFollowCamera (Variables|Default|GetAshe)))) "1.000000,1.000000,1.000000") "Undefined" "MultiplyWithRoot" 0 0))

(event Custom|ResetBase)

(event Custom|ReloadCooldown
  (bind _ashe (Variables|Default|GetAshe))
  (bind _ashe_2 (Variables|Default|GetAshe))
  ;[0.3763 0.0185 0.04092 0.5373 20] RELOAD
  (Variables|Default|SetIsReloading false)
  (Utilities|FlowControl|DoOnce false) ; enters at Reset
)

(event Custom|ProjectUltimate
  ;[0.3763 0.0185 0.04092 0.5373] SPAWN DE PROYECTILES ROTACION Y DIRECCION ultimate
  (Game|SpawnActorfromClass "/Game/MyAssets/BP_Projectile.BP_Projectile_C" (Math|Transform|MakeTransform (Transformation|GetWorldLocation (Variables|Default|GetMuzzle)) (Math|Conversions|RotationFromXVector (Math|Vector|GetForwardVector (Variables|/Game/ThirdPerson/Blueprints/BP_ThirdPersonCharacter.BP_ThirdPersonCharacter_C|GetFollowCamera (Variables|Default|GetAshe)))) "1.000000,1.000000,1.000000") "Undefined" "MultiplyWithRoot" 0 0))

(event Custom|ResetUltimate)

(event EventBeginPlay
  (bind _asbp_third_person_character (Utilities|Casting|CastToBP_ThirdPersonCharacter (Game|GetPlayerCharacter 0)))
  (Variables|Default|SetAshe _asbp_third_person_character))

(event Collision|EventActorBeginOverlap
  (params (OtherActor :type Actor%20Object%20Reference)))

(event EventAttackBasic
  ;[0.3763 0.0185 0.04092 0.5373] Attack Basic
  (Development|PrintString "BASIC")
  (if (< (Variables|Default|GetAttackBasic_Count) 3)
    (CallFunction|ProjectileBasic)
    (Math|Integer|IncrementInt (Variables|Default|GetAttackBasic_Count)
      (:%20%20
        (Utilities|FlowControl|RetriggerableDelay 2.0)
        (Variables|Default|SetAttackBasic_Count 0)))
    (else
      (|TripleShoot)
      (Variables|Default|SetAttackBasic_Count 0))))

(event EventAttackSpecial
  (bind _ashe (Variables|Default|GetAshe))
  (bind _followcamera (Variables|/Game/ThirdPerson/Blueprints/BP_ThirdPersonCharacter.BP_ThirdPersonCharacter_C|GetFollowCamera _ashe))
  ;[0.3763 0.0185 0.04092 0.5373] Attack Special
  (Development|PrintString "SPECIAL")
  (Variables|Default|SetAttackSpecial_CurrentRotaion (* (/ (* (- (Variables|Default|GetAttackSpecial_Count) 1) (Variables|Default|GetAttackSpecial_Angle)) 2.0) -1.0))
  (for _index (range 1 (Variables|Default|GetAttackSpecial_Count))
    (Game|SpawnActorfromClass "/Game/MyAssets/BP_Projectile.BP_Projectile_C" (Math|Transform|MakeTransform (Transformation|GetWorldLocation (Variables|Default|GetMuzzle)) (Math|Conversions|RotationFromXVector (Math|Vector|RotateVectorAroundAxis (Math|Vector|GetForwardVector _followcamera) (Variables|Default|GetAttackSpecial_CurrentRotaion) (Math|Vector|GetUpVector _followcamera))) "1.000000,1.000000,1.000000") "Undefined" "MultiplyWithRoot" 0 0)
    (Variables|Default|SetAttackSpecial_CurrentRotaion (+ (Variables|Default|GetAttackSpecial_CurrentRotaion) (Variables|Default|GetAttackSpecial_Angle)))))

(event EventAttackUltimate
  ;[0.3763 0.0185 0.04092 0.5373] Attack Ultimate
  (Development|PrintString "ULTIMATE")
  (CallFunction|ProjectUltimate))

(event EventTick
  (params (DeltaSeconds :type Float%20%28single-precision%29)))

(event EventShoot
  (params (AttackTipe :type Enum_AttackTipe%20Enum :default "NewEnumerator0"))
  ;[0.3763 0.0185 0.04092 0.5373] Shoot
  (if (not (Variables|Default|GetIsReloading))
    (switch Utilities|FlowControl|Switch|SwitchonEnum_AttackTipe AttackTipe
      (:NewEnumerator0
        (Utilities|FlowControl|DoOnce false :!label _label
          (:Completed
            (Utilities|CheckAmmo (Variables|Default|GetAttackBasic_Cost)
              (:OK
                (CallFunction|AttackBasic))
              (:Denied
                _))
            (Utilities|FlowControl|Delay (Variables|Default|GetAttack_Basic_CoolDown))
            (goto _label Reset))))
      (:NewEnumerator1
        (Utilities|FlowControl|DoOnce false :!label _label_2
          (:Completed
            (Utilities|CheckAmmo (Variables|Default|GetAttackSpecial_Cost)
              (:OK
                (CallFunction|AttackSpecial))
              (:Denied
                _))
            (Utilities|FlowControl|Delay (Variables|Default|GetAttack_Special_CoolDown))
            (goto _label_2 Reset))))
      (:NewEnumerator2
        (Utilities|FlowControl|DoOnce false :!label _label_3
          (:Completed
            (Utilities|CheckAmmo (Variables|Default|GetAttackUltimate_Cost)
              (:OK
                (CallFunction|AttackUltimate))
              (:Denied
                _))
            (Utilities|FlowControl|Delay (Variables|Default|GetAttack_Ultimate_CoolDown))
            (goto _label_3 Reset)))))))

(event EventReload
  (bind _ashe (Variables|Default|GetAshe))
  (bind _ashe_2 (Variables|Default|GetAshe))
  ;[0.3763 0.0185 0.04092 0.5373 20] RELOAD
  (if (and (< (Variables|Default|GetAmmoCurrent) (Variables|Default|GetAmmoMax)) (not (Variables|/Game/ThirdPerson/Blueprints/BP_ThirdPersonCharacter.BP_ThirdPersonCharacter_C|GetIsAiming (Variables|Default|GetAshe))))
    (Utilities|FlowControl|DoOnce false
      (:Completed
        (Variables|Default|SetIsReloading true)
        (Variables|Default|SetAmmoNeeded (- (Variables|Default|GetAmmoMax) (Variables|Default|GetAmmoCurrent)))
        (if (>= (Variables|/Game/ThirdPerson/Blueprints/BP_ThirdPersonCharacter.BP_ThirdPersonCharacter_C|GetAmmo (Variables|Default|GetAshe)) (Variables|Default|GetAmmoNeeded))
          (Utilities|FlowControl|Delay 1.5)
          (Variables|Default|SetAmmoCurrent (Variables|Default|GetAmmoMax))
          (Variables|/Game/ThirdPerson/Blueprints/BP_ThirdPersonCharacter.BP_ThirdPersonCharacter_C|SetAmmo _ashe (- (Variables|/Game/ThirdPerson/Blueprints/BP_ThirdPersonCharacter.BP_ThirdPersonCharacter_C|GetAmmo _ashe) (Variables|Default|GetAmmoNeeded)))
          (Development|PrintString "Reloaded Full Charger")
          (elif (> (Variables|/Game/ThirdPerson/Blueprints/BP_ThirdPersonCharacter.BP_ThirdPersonCharacter_C|GetAmmo (Variables|Default|GetAshe)) 0)
            (Variables|Default|SetAmmoCurrent (+ (Variables|Default|GetAmmoCurrent) (Variables|/Game/ThirdPerson/Blueprints/BP_ThirdPersonCharacter.BP_ThirdPersonCharacter_C|GetAmmo _ashe_2)))
            (Variables|/Game/ThirdPerson/Blueprints/BP_ThirdPersonCharacter.BP_ThirdPersonCharacter_C|SetAmmo _ashe_2 0)
            (Development|PrintString "Reloaded Partial Charger")
            (else
              (Development|PrintString "CHARGER NO RELOAD NO AMMO"))))
        (CallFunction|ReloadCooldown)))))

(fn ConstructionScript)