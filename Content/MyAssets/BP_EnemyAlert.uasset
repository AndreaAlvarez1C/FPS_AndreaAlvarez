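; Short-lived alert actor that spreads outward from its location and makes enemies it reaches call Cry.
; On BeginPlay the AlertExpansion timeline, with play rate set to the inverse of Duration, lerps the sphere radius while updating overlaps.
; Actor overlaps trigger Cry only on actors whose class is exactly BP_Enemy, excluding subclasses.
; The actor destroys itself when the timeline finishes.
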(event EventBeginPlay
  ;[0.104 0.1993 0.3438 0.4] Hace la animación más lenta
  (Components|Timeline|SetPlayRate (Variables|Default|GetAlertExpansion) (/ 1.0 (Variables|Default|GetDuration)))
  (bind _alpha (Timeline|AlertExpansion Play)
    (:Update
      ;[0.15 0.15 0.15 0.5] Hace que crezca el radio de la esfera
      (Components|Sphere|SetSphereRadius (Variables|Default|GetSphere) (Math|Float|Lerp 32.0 2e+03 _alpha) true))
    (:Finished
      (Actor|DestroyActor))))

(event Collision|EventActorBeginOverlap
  (params (OtherActor :type Actor%20Object%20Reference))
  ;[0.15 0.15 0.15 0.5 12] Para detectar enemigos y que hagan el Cry
  (if (== (Utilities|GetClass OtherActor) "/Game/MyAssets/BP_Enemy.BP_Enemy_C")
    (bind _asbp_enemy (Utilities|Casting|CastToBP_Enemy OtherActor))
    (Default|Cry _asbp_enemy)))

(event EventTick
  (params (DeltaSeconds :type Float%20%28single-precision%29)))

(fn ConstructionScript)