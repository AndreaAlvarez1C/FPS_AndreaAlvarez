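; Vel'Koz enemy that patrols, roams or guards around a PatrolPoint until it gains aggro on the player character.
; Seeing the player or being shot raises an alert that spawns BP_EnemyAlert, then chains a chase into cooldown-gated projectile attacks.
; A retriggerable delay on each sighting drops aggro and restores the base behaviour when sightings stop.
; Health reaching zero plays a random death montage with a material dissolve, then destroys the actor.
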(event OnSeePawn(PawnSensing)
  (params (Pawn :type Pawn%20Object%20Reference))
  ;[1 0.3325 0.3763 0.5373 32] PAWN
  ;;[0.3763 0.0185 0.04092 0.5373] PAWN SENSING
  (if (== Pawn (Variables|Default|GetAshe))
    (CallFunction|TryNotSeePawn)
    (if (not (Variables|Default|GetHasAggro))
      (CallFunction|BehaviourAlert))))

(event Custom|LaunchBaseBehaviour
  ;[0.3763 0.0185 0.04092 0.5373] Activación de estados
  (switch Utilities|FlowControl|Switch|SwitchonEnum_EnemyStates (Variables|Default|GetBaseBehaviour)
    (:NewEnumerator0
      (CallFunction|BehaviourPatrol))
    (:NewEnumerator1
      (CallFunction|BehaviourRoam))
    (:NewEnumerator2
      (CallFunction|BehaviourGuard))))

(event Custom|Behaviour_Guard
  ;[0.143 0.15 0.01328 0.5] ESTADOS
  ;;[0.3763 0.0185 0.04092 0.5373] GUARD
  (if (not (Variables|Default|GetHasAggro))
    ;;;[0.008396 0.2485 0.3333 0.5913 12] Va hacia dónde esté el Patrolpoint
    (AI|AIMoveTo self "0, 0, 0" (Variables|Default|GetPatrolPoint) 1.0 false
      (:OnSuccess
        ;;;[0.09095 0.1455 0.3333 0.5913 14] Transición de rotación para que el enemy se ponga en la misma dirección que el patrolpoint
        (Variables|Default|SetGuard_InitialRotation (Transformation|GetActorRotation))
        (Variables|Default|SetGuard_EndRotation (Transformation|GetActorRotation (Variables|Default|GetPatrolPoint)))
        ;;;;[0.3763 0.2931 0.05671 0.5373 10] Animación de traslación de rotación
        (bind _alpha (Timeline|Guard_RotationAnimation Play)
          (:Update
            (Transformation|SetActorRotation (Math|Rotator|Lerp(Rotator) (Variables|Default|GetGuard_InitialRotation) (Variables|Default|GetGuard_EndRotation) _alpha true))))))))

(event Custom|ResetAttack
  ;[1 0.3325 0.3763 0.5373 32] BEHAVIOUR
  ;;[0.3763 0.0185 0.04092 0.5373] BehaviourAttack
  (Utilities|FlowControl|DoOnce false) ; enters at Reset
)

(event Custom|BehaviourAlert
  ;[1 0.3325 0.3763 0.5373 32] BEHAVIOUR
  ;;[0.3763 0.0185 0.04092 0.5373] BEHAVIOUR ALERT
  (Utilities|FlowControl|DoOnce false
    (:Completed
      (Variables|Default|SetHasAggro true)
      (CallFunction|BehaviourStop)
      (Game|SpawnActorfromClass "/Game/MyAssets/BP_EnemyAlert.BP_EnemyAlert_C" (Math|Transform|MakeTransform (Transformation|GetActorLocation) "0, 0, 0" "1.000000,1.000000,1.000000") "Undefined" "MultiplyWithRoot" 0 0)
      (bind _returnvalue (Animation|PlayAnimMontage "/Game/Characters/VelKoz/Animations/AM_Velkoz_Alert.AM_Velkoz_Alert" 1.0 "None"))
      (Utilities|FlowControl|Delay _returnvalue)
      (CallFunction|BehaviourChase))))

(event Custom|ResetAlert
  ;[1 0.3325 0.3763 0.5373 32] BEHAVIOUR
  ;;[0.3763 0.0185 0.04092 0.5373] BEHAVIOUR ALERT
  (Utilities|FlowControl|DoOnce false) ; enters at Reset
)

(event Custom|TryNotSeePawn
  ;[1 0.3325 0.3763 0.5373 32] PAWN
  ;;[0.3763 0.0185 0.04092 0.5373] TryNotSeePawn
  (Utilities|FlowControl|RetriggerableDelay 5.0)
  (CallFunction|BehaviourStop)
  (Variables|Default|SetHasAggro false)
  (CallFunction|ResetAlert)
  (Utilities|FlowControl|Delay 2.0)
  (if (not (Variables|Default|GetHasAggro))
    (CallFunction|LaunchBaseBehaviour)))

(event Custom|RedirectAttack
  ;[0.3763 0.0185 0.04092 0.5373] RedirectAttack
  (Transformation|SetActorRotation (Math|Rotator|FindLookatRotation (Transformation|GetActorLocation) (Transformation|GetActorLocation (Variables|Default|GetAshe)))))

(event Custom|Behaviour_Patrol
  ;[0.143 0.15 0.01328 0.5] ESTADOS
  ;;[0.3763 0.0185 0.04092 0.5373] PATROL
  (if (not (Variables|Default|GetHasAggro))
    ;;;[0.104 0.1993 0.3438 0.4 12] Movimiento hacia el punto
    (AI|AIMoveTo self "0, 0, 0" (Variables|Default|GetPatrolPoint) 5.0 false
      (:OnSuccess
        ;;;[0.104 0.1993 0.3438 0.4 12] El tiempo en el que se queda en el punto
        (Utilities|FlowControl|Delay (Math|Random|RandomFloatinRange 2.0 5.0))
        ;;;[0.104 0.1993 0.3438 0.4 12] Para marcar el siguiente punto como al que está llegando
        (Variables|Default|SetPatrolPoint (Variables|/Game/MyAssets/BP_Patrolpoint.BP_Patrolpoint_C|GetNextPatrolPoint (Variables|Default|GetPatrolPoint)))
        (CallFunction|BehaviourPatrol)))))

(event Custom|BehaviourRoam
  ;[0.143 0.15 0.01328 0.5] ESTADOS
  ;;[0.3763 0.0185 0.04092 0.5373] ROAM
  (if (not (Variables|Default|GetHasAggro))
    ;;;[0.104 0.1993 0.3438 0.4 12] Cogerá un punto aleatorio
    (bind _randomlocation (Class|NavigationSystemV1|GetRandomLocationinNavigableRadius (Transformation|GetActorLocation (Variables|Default|GetPatrolPoint)) (Variables|Default|GetRoamRadius) 0 0))
    (if (> (Math|Vector|Distance(Vector) _randomlocation (Transformation|GetActorLocation)) 2e+02)
      ;;;[0.08416 0.1251 0.3438 0.4 12] Hará que se mueva a ese punto
      (AI|AIMoveTo self _randomlocation 0 5.0 false)
      (else
        (CallFunction|BehaviourRoam)))))

(event Custom|Death
  ;[0.3763 0.0185 0.04092 0.5373] Death
  (Utilities|FlowControl|DoOnce false
    (:Completed
      (Pawn|Components|CharacterMovement|SetMovementMode (Variables|Character|GetCharacterMovement) "MOVE_None" 0)
      (bind _returnvalue (Animation|PlayAnimMontage (.OutItem (Utilities|Array|Random (Variables|Default|GetAnim_Death))) 1.0 "None"))
      (bind _dissolve (Timeline|Dissolve PlayFromStart)
        (:Update
          (Rendering|Material|SetScalarParameterValueonMaterials (Variables|Character|GetMesh) "Dissolve" (Math|Float|Lerp -1.0 1.0 _dissolve)))
        (:Finished
          (Utilities|FlowControl|Delay _returnvalue)
          (Actor|DestroyActor))))))

(event Custom|Cry
  ;[0.3763 0.0185 0.04092 0.5373] Cry Alarm
  (if (not (Variables|Default|GetHasAggro))
    (Variables|Default|SetHasAggro true)
    (CallFunction|BehaviourStop)
    (bind _returnvalue (Animation|PlayAnimMontage "/Game/Characters/Fiddlesticks/Animation/AM_Fiddlesticks_Cry.AM_Fiddlesticks_Cry" 1.0 "None"))
    (Utilities|FlowControl|Delay _returnvalue)
    (CallFunction|BehaviourChase)))

(event Custom|BehaviourChase
  ;[1 0.3325 0.3763 0.5373 32] BEHAVIOUR
  ;;[0.3763 0.0185 0.04092 0.5373] BehaviourChase
  (AI|AIMoveTo self "0, 0, 0" (Variables|Default|GetAshe) (Variables|Default|GetAttackDistance) false
    (:OnSuccess
      (Development|PrintString "CHASE VELKOZ")
      (CallFunction|BehaviourAttack))))

(event Custom|BehaviourAttack
  ;[1 0.3325 0.3763 0.5373 32] BEHAVIOUR
  ;;[0.3763 0.0185 0.04092 0.5373] BehaviourAttack
  (Utilities|FlowControl|DoOnce false
    (:Completed
      ;;;[0.15 0.15 0.15 0.5 12] Ataque de lejos
      (Animation|PlayAnimMontage "/Game/Characters/VelKoz/Animations/AM_Velkoz_Attack.AM_Velkoz_Attack" 1.0 "None")
      (Development|PrintString "ATTACK FAR")
      (CallFunction|Projectile)
      (Utilities|FlowControl|Delay (Variables|Default|GetAttackCooldown))
      (CallFunction|ResetAttack)
      (CallFunction|BehaviourChase))))

(event Custom|BehaviourStop
  (bind _self self)
  ;[1 0.3325 0.3763 0.5373 32] BEHAVIOUR
  ;;[0.3763 0.0185 0.04092 0.5373] BehaviourStop
  ;;;[0.104 0.1993 0.3438 0.4 12] Hará que se para ya que el sitio dónde debe ir es su posición actual
  (AI|AIMoveTo _self "0, 0, 0" _self 5.0 false))

(event Custom|Projectile
  ;[0.3763 0.0185 0.04092 0.5373] Projectile
  (CallFunction|RedirectAttack)
  (Game|SpawnActorfromClass "/Game/MyAssets/BP_ProjectileVelkoz.BP_ProjectileVelkoz_C" (Math|Transform|MakeTransform (Transformation|GetWorldLocation (Variables|Default|GetProjectileVelkoz)) (Math|Conversions|RotationFromXVector (Math|Vector|GetForwardVector (Variables|Collision|GetCapsuleComponent))) "1.000000,1.000000,1.000000") "Undefined" "MultiplyWithRoot" 0 0))

(event EventBeginPlay
  ;[0.3763 0.0185 0.04092 0.5373] BEGIN PLAYS
  (CallFunction|LaunchBaseBehaviour)
  (bind _asbp_third_person_character (Utilities|Casting|CastToBP_ThirdPersonCharacter (Game|GetPlayerCharacter 0)))
  (Variables|Default|SetAshe _asbp_third_person_character))

(event Collision|EventActorBeginOverlap
  (params (OtherActor :type Actor%20Object%20Reference)))

(event EventTick
  (params (DeltaSeconds :type Float%20%28single-precision%29)))

(event EventOnShot
  (params (DirectionShoot :type Vector :default "0, 0, 0") (Damage :type Float%20%28double-precision%29))
  ;[0.3763 0.0185 0.04092 0.5373] OnShot
  (Utilities|HealthManager Damage
    (:IsDead
      (CallFunction|Death))
    (:IsAlive
      (if (not (Variables|Default|GetHasAggro))
        (Utilities|FlowControl|DoOnce false
          (:Completed
            (CallFunction|BehaviourAlert)))))))

(fn ConstructionScript)